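; Story Framework save manager component that saves and loads game progress through one SFSaveGame_BP slot, with optional interval autosave outside the main menu.
; Saving gathers player transform, camera, inventory, journal, tasks and dialogue state from manager components, plus world changes, sequences and NPC data, then shows a popup.
; Loading restores these, replaying spawned, destroyed and interacted actors per level, matching existing actors by object name and NPCs by ID.
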(event `self.ReceiveBeginPlay`
  (bind _storyframeworkvalues (`/Game/StoryFramework/Core/Blueprints/BlueprintLibraries/SFGameplayFunctions_BFL.GetCurrentSFV (Instance)`))
  ;[1 0.2588 0] Save method control
  (`/Engine/EditorBlueprintResources/StandardMacros.IsValid` _storyframeworkvalues
    (:`Is Valid`
      (switch `/Game/StoryFramework/Core/Blueprints/Enumerators/SaveMethod_E` (`/Game/StoryFramework/Core/Blueprints/DataAssets/SFCustomization_PDA.SaveMethod` _storyframeworkvalues)
        (:`NewEnumerator0`
          (`self.AutoSave (StoryFramework)`))
        (:`NewEnumerator1`)))
    (:`Is Not Valid`)))

(event `AutoSave (StoryFramework)`
  ;[0.04314 0.04314 0.05098] Systems (Root)
  (`KismetSystemLibrary.K2_SetTimer` null "AutoSaveLoop" (`/Game/StoryFramework/Core/Blueprints/DataAssets/SFCustomization_PDA.AutoSaveIntervals` (`/Game/StoryFramework/Core/Blueprints/BlueprintLibraries/SFGameplayFunctions_BFL.GetCurrentSFV (Instance)`)) true))

(event `AutoSaveLoop`
  ;[0.04314 0.04314 0.05098] Systems (Root)
  (if (not (`KismetStringLibrary.Contains` (`KismetSystemLibrary.GetDisplayName` (`GameplayStatics.GetGameMode`)) "MainMenu_GM"))
    (`self.SaveGame (StoryFramework)`)))

(event `SaveGame (StoryFramework)`
  (bind _interactionmanager (`/Game/StoryFramework/Core/Blueprints/BlueprintLibraries/SFGameplayFunctions_BFL.GetSFInteractionManager (Controller)`))
  (bind _inventorymanager (`/Game/StoryFramework/Core/Blueprints/BlueprintLibraries/SFGameplayFunctions_BFL.GetSFInventoryManager (Controller)`))
  (bind _inventorymanager_2 (`/Game/StoryFramework/Core/Blueprints/BlueprintLibraries/SFGameplayFunctions_BFL.GetSFInventoryManager (Controller)`))
  (bind _cameramanager (`/Game/StoryFramework/Core/Blueprints/BlueprintLibraries/SFGameplayFunctions_BFL.GetSFCameraManager (Controller)`))
  (bind _sequencemanager (`/Game/StoryFramework/Core/Blueprints/BlueprintLibraries/SFGameplayFunctions_BFL.GetSFSequenceManager (Controller)`))
  (bind _playertransform (`self.PlayerTransform`))
  (bind _assfgame_instance_bp (cast `/Game/StoryFramework/Core/SFGameInstance_BP` (`GameplayStatics.GetGameInstance`) :!pure true))
  ;[0.04314 0.04314 0.05098] Systems (Root)
  (bind _returnvalue (`GameplayStatics.CreateSaveGameObject` "/Game/StoryFramework/SaveGame/SFSaveGame_BP.SFSaveGame_BP_C"))
  (bind _returnvalue_2 (`GameplayStatics.GetCurrentLevelName` true))
  (`BlueprintMapLibrary.Map_Add` _playertransform (`KismetStringLibrary.Conv_StringToName` _returnvalue_2) (`Actor.GetTransform` (`GameplayStatics.GetPlayerCharacter` 0)))
  (set `/Game/StoryFramework/SaveGame/SFSaveGame_BP.PlayerTransform` _playertransform _returnvalue)
  (set `/Game/StoryFramework/SaveGame/SFSaveGame_BP.InventoryItems` (`/Game/StoryFramework/Core/Blueprints/Components/Core/SFInventoryManager_AC.InventoryItems` _inventorymanager) _returnvalue) ; Save inventory.
  (set `/Game/StoryFramework/SaveGame/SFSaveGame_BP.InventoryItemData` (`/Game/StoryFramework/Core/Blueprints/Components/Core/SFInventoryManager_AC.InventoryItemData` _inventorymanager) _returnvalue)
  (`/Engine/EditorBlueprintResources/StandardMacros.IsValid` (`/Game/StoryFramework/Core/Blueprints/BlueprintLibraries/SFCameraGeneralFunctions_BFL.GetSFCameraComponentFromCharacter` 0)
    (:`Is Valid`
      (set `/Game/StoryFramework/SaveGame/SFSaveGame_BP.CameraSettings` (make `/Game/StoryFramework/SaveGame/Blueprints/Structures/CameraSaveData_S` (`/Game/StoryFramework/Core/Blueprints/Components/Core/SFCameraManager_AC.FirstPersonCameraPreset` _cameramanager) (`/Game/StoryFramework/Core/Blueprints/Components/Core/SFCameraManager_AC.ThirdPersonCameraPreset` _cameramanager) (`/Game/StoryFramework/Core/Blueprints/Components/Other/SFDefaultCamera_CC.CurrentCameraPreset` (`/Game/StoryFramework/Core/Blueprints/BlueprintLibraries/SFCameraGeneralFunctions_BFL.GetSFCameraComponentFromCharacter` 0))) _returnvalue) ; Save camera settings.
    )
    (:`Is Not Valid`
      _))
  (set `/Game/StoryFramework/SaveGame/SFSaveGame_BP.ControlRotation` (`Controller.GetControlRotation` (`GameplayStatics.GetPlayerController` 0)) _returnvalue) ; Save player rotation.
  (set `/Game/StoryFramework/SaveGame/SFSaveGame_BP.JournalEntries` (`/Game/StoryFramework/Core/Blueprints/Components/Core/SFInventoryManager_AC.JournalEntries` (`/Game/StoryFramework/Core/Blueprints/BlueprintLibraries/SFGameplayFunctions_BFL.GetSFInventoryManager (Controller)`)) _returnvalue) ; Save journal entries.
  (set `/Game/StoryFramework/SaveGame/SFSaveGame_BP.ConsequentialTags` (`/Game/StoryFramework/Core/Blueprints/Components/Core/SFInteractionManager_AC.ConsequentialTags` (`/Game/StoryFramework/Core/Blueprints/BlueprintLibraries/SFGameplayFunctions_BFL.GetSFInteractionManager (Controller)`)) _returnvalue) ; Save NPC dialog tags.
  (set `/Game/StoryFramework/SaveGame/SFSaveGame_BP.PlayerTasks` (`/Game/StoryFramework/Core/Blueprints/Components/Core/SFInventoryManager_AC.AllPlayerTasks` _inventorymanager_2) _returnvalue) ; Save player Tasks
  (set `/Game/StoryFramework/SaveGame/SFSaveGame_BP.TrackedTask` (`/Game/StoryFramework/Core/Blueprints/Components/Core/SFInventoryManager_AC.TrackedTask` _inventorymanager_2) _returnvalue)
  (set `/Game/StoryFramework/SaveGame/SFSaveGame_BP.AddedNPCReplies` (`/Game/StoryFramework/Core/Blueprints/Components/Core/SFInteractionManager_AC.AddedReplies` _interactionmanager) _returnvalue)
  (set `/Game/StoryFramework/SaveGame/SFSaveGame_BP.HiddenNPCReplies` (`/Game/StoryFramework/Core/Blueprints/Components/Core/SFInteractionManager_AC.HiddenReplies` _interactionmanager) _returnvalue)
  (set `/Game/StoryFramework/SaveGame/SFSaveGame_BP.SpawnedActors` (`self.SpawnedActors`) _returnvalue) ; Save spawned actors.
  (set `/Game/StoryFramework/SaveGame/SFSaveGame_BP.InteractActors` (`self.InteractActors`) _returnvalue)
  (bind _returnvalue_3 (`GameplayStatics.GetCurrentLevelName` true))
  (set `/Game/StoryFramework/SaveGame/SFSaveGame_BP.SystemData` (make `/Game/StoryFramework/SaveGame/Blueprints/Structures/SystemSaveData_S` (`KismetMathLibrary.Now`) (`/Game/StoryFramework/Core/SFGameInstance_BP.Sensitivity` _assfgame_instance_bp) (`/Game/StoryFramework/Core/SFGameInstance_BP.MasterVolume` _assfgame_instance_bp) (`KismetStringLibrary.Conv_StringToName` _returnvalue_3)) _returnvalue) ; Save system data info.
  (set `/Game/StoryFramework/SaveGame/SFSaveGame_BP.DestroyedActors` (`self.DestroyedActors`) _returnvalue)
  (`/Engine/EditorBlueprintResources/StandardMacros.IsValid` _sequencemanager
    (:`Is Valid`
      (set `/Game/StoryFramework/SaveGame/SFSaveGame_BP.SavedSequences` (`/Game/StoryFramework/Core/Blueprints/Components/Core/SFSequenceManager_AC.SavedSequences` _sequencemanager) _returnvalue) ; Save completed sequences
    )
    (:`Is Not Valid`
      _))
  (set `/Game/StoryFramework/SaveGame/SFSaveGame_BP.ActorTags` (`self.ActorTags`) _returnvalue)
  (set `/Game/StoryFramework/SaveGame/SFSaveGame_BP.NPCData` (`self.MakeNPCSaveData`) _returnvalue)
  (`GameplayStatics.SaveGameToSlot` _returnvalue "SFSaveSlot")
  (bind _returnvalue_4 (`|CreateWidget` "/Game/StoryFramework/Core/UserInterface/Widgets/PopupMaster_W.PopupMaster_W_C"))
  (`/Game/StoryFramework/Core/UserInterface/Widgets/PopupMaster_W.ShowSavePopup` _returnvalue_4)
  (`UserWidget.AddToViewport` _returnvalue_4 0))

(event `LoadGame (StoryFramework)`
  (params (IgnorePlayerLocation :type Boolean))
  (bind _interactionmanager (`/Game/StoryFramework/Core/Blueprints/BlueprintLibraries/SFGameplayFunctions_BFL.GetSFInteractionManager (Controller)`))
  (bind _inventorymanager (`/Game/StoryFramework/Core/Blueprints/BlueprintLibraries/SFGameplayFunctions_BFL.GetSFInventoryManager (Controller)`))
  (bind _inventorymanager_2 (`/Game/StoryFramework/Core/Blueprints/BlueprintLibraries/SFGameplayFunctions_BFL.GetSFInventoryManager (Controller)`))
  (bind _cameramanager (`/Game/StoryFramework/Core/Blueprints/BlueprintLibraries/SFGameplayFunctions_BFL.GetSFCameraManager (Controller)`))
  (bind _reference (`/Game/StoryFramework/Core/Blueprints/Components/Other/SFDefaultCamera_CC.GetParentSpringArmComponent` (`/Game/StoryFramework/Core/Blueprints/BlueprintLibraries/SFCameraGeneralFunctions_BFL.GetSFCameraComponentFromCharacter` 0) 0))
  (bind _reference_2 (`/Game/StoryFramework/Core/Blueprints/Components/Other/SFDefaultCamera_CC.GetParentSpringArmComponent` (`/Game/StoryFramework/Core/Blueprints/BlueprintLibraries/SFCameraGeneralFunctions_BFL.GetSFCameraComponentFromCharacter` 0) 0))
  ;[0.04314 0.04314 0.05098] Systems (Root)
  (bind _returnvalue (`GameplayStatics.LoadGameFromSlot` "SFSaveSlot"))
  (bind _assfsave_game_bp (cast `/Game/StoryFramework/SaveGame/SFSaveGame_BP` _returnvalue))
  (bind _output_get (set `self.SpawnedActors` (`/Game/StoryFramework/SaveGame/SFSaveGame_BP.SpawnedActors` _assfsave_game_bp)))
  (`|ExecutionSequence`
    (:`then_0`
      (if (`KismetArrayLibrary.Array_IsNotEmpty` _output_get)
        (for _array_element _output_get
          (bind _returnvalue_2 (`GameplayStatics.GetCurrentLevelName` true))
          (bind (_levelname _actorclass _actortransform _actortags _interactabledata _staticmeshactor) (break `/Game/StoryFramework/SaveGame/Blueprints/Structures/LevelActorSaveData_S` _array_element))
          (if (`KismetStringLibrary.EqualEqual_StrStr` (`KismetStringLibrary.Conv_NameToString` _levelname) _returnvalue_2)
            (`/Engine/EditorBlueprintResources/StandardMacros.IsValid` _staticmeshactor
              (:`Is Valid`
                (bind _returnvalue_3 (`|SpawnActorFromClass` "/Script/Engine.StaticMeshActor" _actortransform "Undefined" "OverrideRootScale" null null))
                (bind _staticmeshcomponent (`StaticMeshActor.StaticMeshComponent` _returnvalue_3))
                (`SceneComponent.SetMobility` _staticmeshcomponent "Movable")
                (`StaticMeshComponent.SetStaticMesh` _staticmeshcomponent _staticmeshactor)
                (set `Actor.Tags` _actortags _returnvalue_3))
              (:`Is Not Valid`
                (bind _returnvalue_4 (`|SpawnActorFromClass` _actorclass _actortransform "Undefined" "OverrideRootScale" null null))
                (bind _asinteractable_base_bp (cast `/Game/StoryFramework/Core/Blueprints/InteractableBase_BP` _returnvalue_4))
                (set `/Game/StoryFramework/Core/Blueprints/InteractableBase_BP.InteractionData` _interactabledata _asinteractable_base_bp)
                (`/Game/StoryFramework/Core/Blueprints/InteractableBase_BP.UpdateCosmetics` _asinteractable_base_bp)
                (set `Actor.Tags` _actortags _asinteractable_base_bp)))))))
    (:`then_1`
      (bind _output_get_2 (set `self.DestroyedActors` (`/Game/StoryFramework/SaveGame/SFSaveGame_BP.DestroyedActors` _assfsave_game_bp)))
      (`|ExecutionSequence`
        (:`then_0`
          (bind _returnvalue_5 (`GameplayStatics.GetCurrentLevelName` true))
          (bind _keys (`BlueprintMapLibrary.Map_Keys` _output_get_2))
          (bind (_value _returnvalue_6) (`BlueprintMapLibrary.Map_Find` _output_get_2 (`|GetArrayItem` _keys (`KismetArrayLibrary.Array_Find` _keys (`KismetStringLibrary.Conv_StringToName` _returnvalue_5)))))
          (if _returnvalue_6
            (bind _outactors (`GameplayStatics.GetAllActorsOfClass` "/Script/Engine.Actor"))
            (for _array_element_2 _outactors
              (bind _destroyedactors (break `/Game/StoryFramework/SaveGame/Blueprints/Structures/LevelDestroyedSaveData_S` _value))
              (bind _returnvalue_7 (`KismetSystemLibrary.GetObjectName` _array_element_2))
              (bind _returnvalue_8 (`KismetArrayLibrary.Array_Find` _destroyedactors _returnvalue_7))
              (if (and (`KismetArrayLibrary.Array_Contains` _destroyedactors _returnvalue_7) (> _returnvalue_8 -1))
                (if (`KismetStringLibrary.EqualEqual_StrStr` _returnvalue_7 (`|GetArrayItem` _destroyedactors _returnvalue_8))
                  (`Actor.K2_DestroyActor` _array_element_2))))))
        (:`then_1`
          (bind _output_get_3 (set `self.InteractActors` (`/Game/StoryFramework/SaveGame/SFSaveGame_BP.InteractActors` _assfsave_game_bp)))
          (`|ExecutionSequence`
            (:`then_0`
              (bind _returnvalue_9 (`GameplayStatics.GetCurrentLevelName` true))
              (bind (_value_2 _returnvalue_10) (`BlueprintMapLibrary.Map_Find` _output_get_3 (`KismetStringLibrary.Conv_StringToName` _returnvalue_9)))
              (if _returnvalue_10
                (bind _outactors_2 (`GameplayStatics.GetAllActorsOfClass` "/Script/Engine.Actor"))
                (for _array_element_3 _outactors_2
                  (bind (_value_3 _returnvalue_11) (`BlueprintMapLibrary.Map_Find` (`.InteractActors_4_C8B2A9F140091C23CC881D940E84A020` (break `/Game/StoryFramework/SaveGame/Blueprints/Structures/LevelInteractSaveData_S` _value_2)) (`KismetSystemLibrary.GetObjectName` _array_element_3)))
                  (if _returnvalue_11
                    (bind _asinteractable_base_bp_2 (cast `/Game/StoryFramework/Core/Blueprints/InteractableBase_BP` _array_element_3))
                    (`/Game/StoryFramework/Core/Blueprints/InteractableBase_BP.LoadFromDataString` _asinteractable_base_bp_2 _value_3)))))
            (:`then_1`
              (set `/Game/StoryFramework/Core/Blueprints/Components/Core/SFSequenceManager_AC.SavedSequences` (`/Game/StoryFramework/SaveGame/SFSaveGame_BP.SavedSequences` _assfsave_game_bp) (`/Game/StoryFramework/Core/Blueprints/BlueprintLibraries/SFGameplayFunctions_BFL.GetSFSequenceManager (Controller)`))
              (bind _output_get_4 (set `self.ActorTags` (`/Game/StoryFramework/SaveGame/SFSaveGame_BP.ActorTags` _assfsave_game_bp)))
              (for _array_element_4 _output_get_4
                (bind _outactors_3 (`GameplayStatics.GetAllActorsOfClass` "/Script/Engine.Actor"))
                (for _array_element_5 _outactors_3
                  (bind (_actorname _tags) (break `/Game/StoryFramework/SaveGame/Blueprints/Structures/LevelActorTagSave_S` _array_element_4))
                  (if (`KismetStringLibrary.EqualEqual_StrStr` (`KismetSystemLibrary.GetObjectName` _array_element_5) _actorname)
                    (set `Actor.Tags` _tags _array_element_5))))
              (bind _output_get_5 (set `self.NPCData` (`/Game/StoryFramework/SaveGame/SFSaveGame_BP.NPCData` _assfsave_game_bp)))
              (for _array_element_6 _output_get_5
                (bind (_id _displayname _namecolor _dialoguedatatable _conswitching) (break `/Game/StoryFramework/Core/Blueprints/Structures/NPCSaveData_S` _array_element_6))
                (bind _foundnpc (`/Game/StoryFramework/Core/Blueprints/BlueprintLibraries/SFGameplayFunctions_BFL.GetTargetNPCByID` _id))
                (`/Engine/EditorBlueprintResources/StandardMacros.IsValid` _foundnpc
                  (:`Is Valid`
                    (bind _npcinfo (message `/Game/StoryFramework/Core/Blueprints/BlueprintInterfaces/DialogueInfo_BPI.GetOwnerDialogueData` _foundnpc))
                    (bind _structout (setmembers `/Game/StoryFramework/Core/Blueprints/Structures/NPCBasicInfo_S` :`StructRef` _npcinfo :`NameInfo` (make `/Game/StoryFramework/Core/Blueprints/Structures/NPCBIName_S` _id _displayname _namecolor) :`DialogueDataTable` _dialoguedatatable :`ConsequentialSwitching` _conswitching))
                    (message `/Game/StoryFramework/Core/Blueprints/BlueprintInterfaces/DialogueInfo_BPI.UpdateOwnerDialogueData` _foundnpc _structout))))
              (if (not IgnorePlayerLocation)
                (bind _output_get_6 (set `self.PlayerTransform` (`/Game/StoryFramework/SaveGame/SFSaveGame_BP.PlayerTransform` _assfsave_game_bp)))
                (bind _returnvalue_12 (`GameplayStatics.GetCurrentLevelName` true))
                (bind (_value_4 _returnvalue_13) (`BlueprintMapLibrary.Map_Find` _output_get_6 (`KismetStringLibrary.Conv_StringToName` _returnvalue_12)))
                (if _returnvalue_13
                  (`Actor.K2_SetActorTransform` (`GameplayStatics.GetPlayerCharacter` 0) _value_4 false false) ; Load player location.
                ))
              (`|ExecutionSequence`
                (:`then_0`
                  (`/Engine/EditorBlueprintResources/StandardMacros.IsValid` _reference ; If camera component has spring arm\nparent, disable camera lag
                    (:`Is Valid`
                      (set `SpringArmComponent.bEnableCameraLag` false _reference)
                      (set `SpringArmComponent.bEnableCameraRotationLag` false _reference))
                    (:`Is Not Valid`
                      _))
                  (bind (_firstpersonsettings _thirdpersonsettings _currentcamerapreset) (break `/Game/StoryFramework/SaveGame/Blueprints/Structures/CameraSaveData_S` (`/Game/StoryFramework/SaveGame/SFSaveGame_BP.CameraSettings` _assfsave_game_bp)))
                  (bind _output_get_7 (set `/Game/StoryFramework/Core/Blueprints/Components/Core/SFCameraManager_AC.InitialCameraPreset` _currentcamerapreset _cameramanager))
                  (set `/Game/StoryFramework/Core/Blueprints/Components/Core/SFCameraManager_AC.FirstPersonCameraPreset` _firstpersonsettings _cameramanager)
                  (set `/Game/StoryFramework/Core/Blueprints/Components/Core/SFCameraManager_AC.ThirdPersonCameraPreset` _thirdpersonsettings _cameramanager)
                  (`/Game/StoryFramework/Core/Blueprints/Components/Core/SFCameraManager_AC.UpdateSFCameraPreset` _cameramanager _output_get_7) ; Update camera initial preset
                  (`/Engine/EditorBlueprintResources/StandardMacros.IsValid` _reference_2 ; If camera component has spring arm\nparent, re-enable camera lag
                    (:`Is Valid`
                      (`KismetSystemLibrary.Delay` 0.05)
                      (set `SpringArmComponent.bEnableCameraLag` true _reference_2)
                      (set `SpringArmComponent.bEnableCameraRotationLag` true _reference_2))))
                (:`then_1`
                  (`|ExecutionSequence`
                    (:`then_0`
                      (bind _inventoryitems (`/Game/StoryFramework/SaveGame/SFSaveGame_BP.InventoryItems` _assfsave_game_bp))
                      (bind _keys_2 (`BlueprintMapLibrary.Map_Keys` _inventoryitems))
                      (`/Game/StoryFramework/Core/Blueprints/Components/Core/SFInventoryManager_AC.ClearInventory` _inventorymanager_2)
                      (set `/Game/StoryFramework/Core/Blueprints/Components/Core/SFInventoryManager_AC.InventoryItemData` (`/Game/StoryFramework/SaveGame/SFSaveGame_BP.InventoryItemData` _assfsave_game_bp) (`/Game/StoryFramework/Core/Blueprints/BlueprintLibraries/SFGameplayFunctions_BFL.GetSFInventoryManager (Controller)`))
                      (for _array_element_7 _keys_2
                        (`/Game/StoryFramework/Core/Blueprints/Components/Core/SFInventoryManager_AC.AddItemToInventory` _inventorymanager_2 (`/Game/StoryFramework/Core/Blueprints/Components/Core/SFInventoryManager_AC.GetInventoryItemDataFromName` _inventorymanager_2 _array_element_7) (`BlueprintMapLibrary.Map_Find` _inventoryitems _array_element_7) null)))
                    (:`then_1`
                      (`Controller.SetControlRotation` (`GameplayStatics.GetPlayerController` 0) (`/Game/StoryFramework/SaveGame/SFSaveGame_BP.ControlRotation` _assfsave_game_bp)) ; Load player rotation.
                      (set `/Game/StoryFramework/Core/Blueprints/Components/Core/SFInventoryManager_AC.JournalEntries` (`/Game/StoryFramework/SaveGame/SFSaveGame_BP.JournalEntries` _assfsave_game_bp) (`/Game/StoryFramework/Core/Blueprints/BlueprintLibraries/SFGameplayFunctions_BFL.GetSFInventoryManager (Controller)`))
                      (set `/Game/StoryFramework/Core/Blueprints/Components/Core/SFInteractionManager_AC.ConsequentialTags` (`/Game/StoryFramework/SaveGame/SFSaveGame_BP.ConsequentialTags` _assfsave_game_bp) (`/Game/StoryFramework/Core/Blueprints/BlueprintLibraries/SFGameplayFunctions_BFL.GetSFInteractionManager (Controller)`))
                      (`|ExecutionSequence`
                        (:`then_0`
                          (set `/Game/StoryFramework/Core/Blueprints/Components/Core/SFInventoryManager_AC.AllPlayerTasks` (`/Game/StoryFramework/SaveGame/SFSaveGame_BP.PlayerTasks` _assfsave_game_bp) _inventorymanager)
                          (`/Game/StoryFramework/Core/Blueprints/Components/Core/SFInventoryManager_AC.ForceTrackTask` _inventorymanager (`.TaskHeader_2_AC20336D4C55A0E8F1521490FE820924` (break `/Game/StoryFramework/Core/Blueprints/Structures/TaskInfo_S` (`/Game/StoryFramework/SaveGame/SFSaveGame_BP.TrackedTask` _assfsave_game_bp)))))
                        (:`then_1`
                          (set `/Game/StoryFramework/Core/Blueprints/Components/Core/SFInteractionManager_AC.AddedReplies` (`/Game/StoryFramework/SaveGame/SFSaveGame_BP.AddedNPCReplies` _assfsave_game_bp) _interactionmanager)
                          (set `/Game/StoryFramework/Core/Blueprints/Components/Core/SFInteractionManager_AC.HiddenReplies` (`/Game/StoryFramework/SaveGame/SFSaveGame_BP.HiddenNPCReplies` _assfsave_game_bp) _interactionmanager))))))))))))))

(fn `MakeNPCSaveData`
  (returns (NewNPCData :type "Array of /Game/StoryFramework/Core/Blueprints/Structures/NPCSaveData_S Structure"))
  (`KismetArrayLibrary.Array_Clear` (`self.NPCData`))
  (bind _outactors (`GameplayStatics.GetAllActorsWithInterface` "/Game/StoryFramework/Core/Blueprints/BlueprintInterfaces/DialogueInfo_BPI.DialogueInfo_BPI_C"))
  (for _array_element _outactors
    (bind _npcinfo (message `/Game/StoryFramework/Core/Blueprints/BlueprintInterfaces/DialogueInfo_BPI.GetOwnerDialogueData` _array_element))
    (bind (_nameinfo _dialoguedatatable _consequentialswitching) (break `/Game/StoryFramework/Core/Blueprints/Structures/NPCBasicInfo_S` _npcinfo))
    (bind (_id _displayname _namecolor) (break `/Game/StoryFramework/Core/Blueprints/Structures/NPCBIName_S` _nameinfo))
    (`KismetArrayLibrary.Array_Add` (`self.NPCData`) (make `/Game/StoryFramework/Core/Blueprints/Structures/NPCSaveData_S` _id _displayname _namecolor _dialoguedatatable _consequentialswitching)))
  (return (`self.NPCData`)))