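; MainMenuController_BP is the main menu controller for the story framework, creating the MainMenu_W widget behind a camera fade on BeginPlay.
; It applies the widget menu input mapping and routes select, navigate and back actions to the current menu held by the game instance.
; The first key press advances the menu state, and each press records gamepad use for the widget.
; A DoOnce on Navigate works around a UE 5.5+ input action issue.
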(fn `UserConstructionScript`)