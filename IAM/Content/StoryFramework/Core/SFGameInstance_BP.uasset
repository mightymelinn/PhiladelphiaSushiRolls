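; StoryFramework's Game Instance, handling saving and loading around level transitions plus global volume and camera sensitivity settings.
; Level events use short delays around save manager calls, with OpenLevelSave chaining save, level open and load.
; These events clear the current menu and collect garbage; the standalone save/load ones also reapply camera sensitivity.
; Master volume overrides a base sound mix, clamped above zero so sounds keep playing.
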(fn `GetSFGameInstance`
  (returns (SFGameInstance :type "/Game/StoryFramework/Core/SFGameInstance_BP Object Reference"))
  (return self))