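; Inspect actor that displays an item in 3D through a scene capture so it can be rotated during inspection.
; On creation it shows either a child actor of the item class or a skeletal mesh, falling back to static.
; The capture renders only that object at a given distance.
; The anchor sets the starting rotation, with per-item overrides for meshes, and applies rotation input, doubled on gamepad.
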(event `RotateComponent`
  (params (Direction :type "Vector2D Structure"))
  (bind (_x _y) (`KismetMathLibrary.BreakVector2D` (select `bool` (`/Game/StoryFramework/Core/Blueprints/BlueprintLibraries/SFGameplayFunctions_BFL.IsUsingGamepad`) :`false` Direction :`true` (* Direction (2.0 2.0)))))
  ;[0.04314 0.04314 0.05098] Systems (Root)
  (`SceneComponent.K2_SetRelativeRotation` (`self.Anchor`) (`KismetMathLibrary.ComposeRotators` (`SceneComponent.RelativeRotation` (`self.Anchor`)) (`KismetMathLibrary.MakeRotator` 0.0 (* _y 1.0) (* _x -1.0))) false false))

(event `OnCreated`
  (params (ItemActorClass :type "Actor Class Reference") (ActorDistanceFromCamera :type "Float (double-precision)") (ItemInteractionData :type "/Game/StoryFramework/Core/Blueprints/Structures/InteractableData_S Structure"))
  (bind ((`ObjectName_62_0AB008F3477E2648EFE7F4B99DC53F93` _objectname) (`ObjectStaticMesh_53_EE9024FA467AC4603952289EAC52AD36` _objectstaticmesh) (`ObjectSkeletalMesh_56_134EE34B40B08159C8FC36960741A5BE` _objectskeletalmesh) (`InspectMethodSettings_41_ED16F4484A76885A89642AB9C8F800FF` _inspectmethodsettings)) (break `/Game/StoryFramework/Core/Blueprints/Structures/InteractableData_S` ItemInteractionData))
  (bind _objectscenecapture (`self.ObjectSceneCapture`))
  (bind _rootskm (`self.RootSkM`))
  (bind _objectscenecapture_2 (`self.ObjectSceneCapture`))
  (bind _rootstm (`self.RootStM`))
  (bind _validactorreference (`self.ValidActorReference`))
  (bind (_itemoptions _foundcustomoptions) (`/Game/StoryFramework/Core/Blueprints/Components/Core/SFInteractionManager_AC.GetCustomItemOptionsFromName` (`/Game/StoryFramework/Core/Blueprints/BlueprintLibraries/SFGameplayFunctions_BFL.GetSFInteractionManager (Controller)`) _objectname))
  (bind _childactor (`ChildActorComponent.ChildActor` (`self.ValidActorReference`)))
  ;[0.04314 0.04314 0.05098] Systems (Root)
  (`|ExecutionSequence`
    (:`then_0`
      (if (not (`KismetSystemLibrary.IsValidClass` ItemActorClass))
        (`/Engine/EditorBlueprintResources/StandardMacros.IsValid` _objectskeletalmesh
          (:`Is Valid`
            (`SkeletalMeshComponent.SetSkeletalMeshAsset` _rootskm _objectskeletalmesh)
            (`SceneComponent.SetVisibility` _rootskm true false))
          (:`Is Not Valid`
            (`StaticMeshComponent.SetStaticMesh` _rootstm _objectstaticmesh)
            (`SceneComponent.SetVisibility` _rootstm true false)))
        (`SceneComponent.K2_SetRelativeLocation` (`self.RootStM`) (`.InspectActorOffset_28_23FCFFAF4597C96B1BD0B38BA2DAB751` (break `/Game/StoryFramework/Core/Blueprints/Structures/IMInspectSettings_S` _inspectmethodsettings)) false false)
        (`SceneComponent.K2_SetRelativeLocation` (`self.RootSkM`) (`.InspectActorOffset_28_23FCFFAF4597C96B1BD0B38BA2DAB751` (break `/Game/StoryFramework/Core/Blueprints/Structures/IMInspectSettings_S` _inspectmethodsettings)) false false)
        (`SceneComponent.K2_SetRelativeLocation` _objectscenecapture_2 (`KismetMathLibrary.MakeVector` (* ActorDistanceFromCamera -1.0)) false false) ; Set Scene Capture Component location\nfrom "3DInspectActorDistanceFromCamera"
        (`SceneCaptureComponent.ShowOnlyComponent` _objectscenecapture_2 (select `bool` (`KismetSystemLibrary.IsValid` _objectskeletalmesh) :`false` (`self.RootStM`) :`true` (`self.RootSkM`) :!type "PrimitiveComponent Object Reference"))
        (`SceneComponent.K2_SetRelativeRotation` (`self.Anchor`) (`KismetMathLibrary.SelectRotator` (`.ItemRotationOnInspect_7_225D2065414315A1D95290A90BD6D679` (break `/Game/StoryFramework/Core/Blueprints/Structures/MoreItemOptions_S` _itemoptions)) (struct :`Pitch` 50.0 :`Yaw` -35.0) _foundcustomoptions) false false)
        (`/Engine/EditorBlueprintResources/StandardMacros.IsValid` _validactorreference
          (:`Is Valid`
            (`ActorComponent.K2_DestroyComponent` _validactorreference)))
        (else
          (`/Engine/EditorBlueprintResources/StandardMacros.IsValid` (`self.ValidActorReference`)
            (:`Is Valid`
              (`ChildActorComponent.SetChildActorClass` (`self.ValidActorReference`) ItemActorClass) ; Dont create a new child actor if one already\nexists. Just update.
            )
            (:`Is Not Valid`
              (bind _returnvalue (`AddComponent|NODE_AddChildActorComponent-0` :`bManualAttachment` true :`RelativeTransform` (`KismetMathLibrary.Conv_VectorToTransform` (`.InspectActorOffset_28_23FCFFAF4597C96B1BD0B38BA2DAB751` (break `/Game/StoryFramework/Core/Blueprints/Structures/IMInspectSettings_S` (`.InspectMethodSettings_41_ED16F4484A76885A89642AB9C8F800FF` (break `/Game/StoryFramework/Core/Blueprints/Structures/InteractableData_S` ItemInteractionData)))))))
              (`SceneComponent.K2_AttachToComponent` _returnvalue (`self.Anchor`) "None" "SnapToTarget" "SnapToTarget" "KeepRelative" true)
              (`ChildActorComponent.SetChildActorClass` _returnvalue ItemActorClass)
              (set `self.ValidActorReference` _returnvalue)))
          (`SceneComponent.K2_SetRelativeLocation` _objectscenecapture (`KismetMathLibrary.MakeVector` (* ActorDistanceFromCamera -1.0)) false false) ; Set Scene Capture Component location\nfrom "3DInspectActorDistanceFromCamera"
          (`SceneCaptureComponent.ShowOnlyActorComponents` _objectscenecapture _childactor true)
          (`SceneComponent.K2_SetRelativeRotation` (`self.Anchor`) (struct :`Pitch` 50.0 :`Yaw` -35.0) false false)
          (message `/Game/StoryFramework/Core/Blueprints/BlueprintInterfaces/SFInteraction_BPI.UpdateInteractionData` _childactor ItemInteractionData)
          (`SceneComponent.SetVisibility` (`self.RootStM`) false false)
          (`SceneComponent.SetVisibility` (`self.RootSkM`) false false))))))

(fn `UserConstructionScript`)