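; Camera modifier that drives automatic depth of field through post process, except when the view target is tagged StoryChoiceCam.
; A short camera-forward trace sets focal distance, overridden by the inspected actor during anim inspection, with clamped camera-to-player distance as fallback for non-player view targets.
; Traced distances are scaled by post-process quality.
; Sensor width varies blur by view target, trace hit and NPC dialog, while aperture stays constant.
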(fn `BlueprintModifyPostProcess`
  (params (DeltaTime :type "Float (single-precision)"))
  (returns (PostProcessBlendWeight :type "Float (single-precision)") (PostProcessSettings :type "PostProcessSettings Structure"))
  (bind (_returnvalue _isviewtargetplayer) (`/Game/StoryFramework/Core/Blueprints/BlueprintLibraries/SFCameraGeneralFunctions_BFL.GetControllerViewTarget`))
  (bind _returnvalue_2 (`GameplayStatics.GetPlayerCameraManager` 0))
  (bind _interactionmanager (`/Game/StoryFramework/Core/Blueprints/BlueprintLibraries/SFGameplayFunctions_BFL.GetSFInteractionManager (Controller)`))
  (bind _inspectanimactor (`/Game/StoryFramework/Core/Blueprints/Components/Core/SFInteractionManager_AC.InspectAnimActor` _interactionmanager))
  (bind (_start _end) (`/Game/StoryFramework/Core/Blueprints/BlueprintLibraries/SFGeneralFunctions_BFL.GetVectorDistancedFromOrigin` (`Actor.K2_GetActorLocation` _returnvalue_2) (`Actor.GetActorForwardVector` _returnvalue_2) 350.0))
  (if (not (`Actor.ActorHasTag` (`/Game/StoryFramework/Core/Blueprints/BlueprintLibraries/SFCameraGeneralFunctions_BFL.GetControllerViewTarget`) "StoryChoiceCam"))
    (`/Engine/EditorBlueprintResources/StandardMacros.IsValid` (`GameplayStatics.GetPlayerCharacter` 0)
      (:`Is Valid`
        (bind (_outhit _returnvalue_3) (`KismetSystemLibrary.LineTraceSingle` _start _end "TraceTypeQuery1" true))
        (`/Engine/EditorBlueprintResources/StandardMacros.IsValid` _inspectanimactor
          (:`Is Valid`
            (if (`/Game/StoryFramework/Core/Blueprints/Components/Core/SFInteractionManager_AC.IsAnimInspecting` _interactionmanager)
              (set `self.DoFTraceEnd` (`Actor.K2_GetActorLocation` _inspectanimactor))
              (else
                (set `self.DoFTraceEnd` (`/Game/StoryFramework/Core/Blueprints/BlueprintLibraries/SFTraceResults_BFL.Get Location` _outhit) :!label _label))))
          (:`Is Not Valid`
            (goto _label)))
        (bind _returnvalue_4 (`GameUserSettings.GetGameUserSettings`))
        (bind _returnvalue_5 (* (`/Game/StoryFramework/Core/Blueprints/BlueprintLibraries/SFGeneralFunctions_BFL.GetDistanceBetweenVectors` (`self.DoFTraceEnd`) (`Actor.K2_GetActorLocation` (`GameplayStatics.GetPlayerCameraManager` 0))) (select `int` (`GameUserSettings.GetPostProcessingQuality` _returnvalue_4) :`0` 1.1 :`1` 1.1 :`2` 1.1 :`3` 1.0 :`4` 1.0)))
        (set `self.FocalDistance` (`KismetMathLibrary.SelectFloat` _returnvalue_5 (`KismetMathLibrary.SelectFloat` _returnvalue_5 (`KismetMathLibrary.SelectFloat` 0.0 (`KismetMathLibrary.FClamp` (`/Game/StoryFramework/Core/Blueprints/BlueprintLibraries/SFGeneralFunctions_BFL.GetDistanceBetweenVectors` (`Actor.K2_GetActorLocation` (`GameplayStatics.GetPlayerCameraManager` 0)) (`Actor.K2_GetActorLocation` (`GameplayStatics.GetPlayerCharacter` 0))) 200.0 1000.0) (`.IsViewTargetPlayer` (`/Game/StoryFramework/Core/Blueprints/BlueprintLibraries/SFCameraGeneralFunctions_BFL.GetControllerViewTarget`))) _returnvalue_3) (`/Game/StoryFramework/Core/Blueprints/Components/Core/SFInteractionManager_AC.IsAnimInspecting` (`/Game/StoryFramework/Core/Blueprints/BlueprintLibraries/SFGameplayFunctions_BFL.GetSFInteractionManager (Controller)`))))
        (set `self.Aperture (F-stop)` 1.5)
        (set `self.Sensor Width (Mm)` (`KismetMathLibrary.SelectFloat` 15.0 (`KismetMathLibrary.SelectFloat` 15.0 (`KismetMathLibrary.SelectFloat` 50.0 100.0 (`/Game/StoryFramework/Core/Blueprints/Components/Core/SFInteractionManager_AC.IsInDialogWithNPC` (`/Game/StoryFramework/Core/Blueprints/BlueprintLibraries/SFGameplayFunctions_BFL.GetSFInteractionManager (Controller)`))) _returnvalue_3) (or _isviewtargetplayer (`Actor.ActorHasTag` _returnvalue "AnimInspect"))))
        (return 1.0 (make `PostProcessSettings` :`DepthOfFieldFstop` (`self.Aperture (F-stop)`) :`DepthOfFieldMinFstop` 11.0 :`DepthOfFieldSensorWidth` (`self.Sensor Width (Mm)`) :`DepthOfFieldFocalDistance` (`self.FocalDistance`)))))))