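; Camera view target for Story Framework left/right choices, presenting the selection visually and running its countdown.
; On begin play it slowly narrows FOV, starts a looping random rotation shake and desaturates through a dynamic post-process material.
; Choice updates animate saturation and the desaturated side, then notify StoryChoice_W.
; A timeline scaled to the timer length feeds the sequence manager controller's timer value and auto-selects on expiry, randomly if nothing is chosen.
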(event `SlightCameraShake`
  (set `self.RandomAdditiveRotation` (`KismetMathLibrary.MakeRotator` (+ (.roll (`self.OriginalCameraRotation`)) (`KismetMathLibrary.RandomFloatInRange` -0.1 0.1)) (+ (.pitch (`self.OriginalCameraRotation`)) (`KismetMathLibrary.RandomFloatInRange` -0.1 0.1)) (+ (.yaw (`self.OriginalCameraRotation`)) (`KismetMathLibrary.RandomFloatInRange` -0.1 0.1))))
  (bind (_direction _alpha) (`Timeline|ShakeCamera` :!via `PlayFromStart`) ; Lerp between randomized rotations.
    (:`Update`
      (`self.K2_SetActorRotation` (`KismetMathLibrary.RLerp` (`self.K2_GetActorRotation`) (`self.RandomAdditiveRotation`) _alpha true)))))

(event `StartTimer`
  (params (Timer :type "Float (double-precision)"))
  (bind _storychoicetimer (`self.StoryChoiceTimer`))
  (`TimelineComponent.SetPlayRate` _storychoicetimer (/ 1.0 Timer)) ; Set length of timer.
  (`TimelineComponent.PlayFromStart` _storychoicetimer))

(event `StopTimer`
  (bind _sequencemanager (`/Game/StoryFramework/Core/Blueprints/BlueprintLibraries/SFGameplayFunctions_BFL.GetSFSequenceManager (Controller)`))
  (bind (_direction _alpha) (`Timeline|StoryChoiceTimer` :!via `Stop`)
    (:`Update`
      (bind _output_get (set `/Game/StoryFramework/Core/Blueprints/Components/Core/SFSequenceManager_AC.ValidTimerValue` (`KismetMathLibrary.Lerp` (`.ChoiceTimer_21_67E9F5B14EFC64549959CA8A9F5A3F02` (break `/Game/StoryFramework/Core/Blueprints/Structures/StoryChoiceData_S` (`/Game/StoryFramework/Core/Blueprints/Components/Core/SFSequenceManager_AC.ValidStoryChoiceData` (`/Game/StoryFramework/Core/Blueprints/BlueprintLibraries/SFGameplayFunctions_BFL.GetSFSequenceManager (Controller)`)))) 0.0 _alpha) (`/Game/StoryFramework/Core/Blueprints/BlueprintLibraries/SFGameplayFunctions_BFL.GetSFSequenceManager (Controller)`))))
    (:`Finished`
      (if (< _output_get 1.0)
        (if (== (`self.CurrentChoiceIndex`) 0)
          (`/Game/StoryFramework/Core/Blueprints/Components/Core/SFSequenceManager_AC.NavigateStoryChoices` _sequencemanager (`KismetMathLibrary.Conv_IntToDouble` (`KismetMathLibrary.SelectInt` -1 1 (`KismetMathLibrary.RandomBool`)))))
        (`/Game/StoryFramework/Core/Blueprints/Components/Core/SFSequenceManager_AC.SelectStoryChoice` _sequencemanager)))))

(event `self.ReceiveBeginPlay`
  ;[0.04314 0.04314 0.05098] Events (Root)
  (bind _asmaterial_interface (cast `MaterialInterface` (`.Object` (break `WeightedBlendable` (`|GetArrayItem` (`.Array` (break `WeightedBlendables` (`.WeightedBlendables` (break `PostProcessSettings` (`CameraComponent.PostProcessSettings` (`self.Camera`)))))))))))
  (bind _returnvalue (`KismetMaterialLibrary.CreateDynamicMaterialInstance` _asmaterial_interface))
  (bind _output_get (set `self.ChoiceDesaturationPPMat` _returnvalue))
  (`MaterialInstanceDynamic.SetScalarParameterValue` _output_get "OverallDesaturation" 1.0)
  (`self.UpdateCameraPostProcessMat` _output_get)
  (`TimelineComponent.PlayFromStart` (`self.SlowFocus`)) ; Slowly focus camera FOV
  (set `self.OriginalCameraRotation` (`self.K2_GetActorRotation`))
  (`KismetSystemLibrary.K2_SetTimer` null "SlightCameraShake" 0.05 true))

(event `UpdateChoice`
  (params (SelectedChoiceIndex :type Integer))
  (bind _fadeppdirection (`self.FadePPDirection`))
  (bind _returnvalue (not (== (`self.CurrentChoiceIndex`) 0)))
  ;[0.04314 0.04314 0.05098] Events (Root)
  (switch `int` SelectedChoiceIndex
    (:`-1`
      (if (not _returnvalue)
        (`TimelineComponent.PlayFromStart` (`self.FadePPSaturation`)))
      (`TimelineComponent.PlayFromStart` _fadeppdirection))
    (:`1`
      (if (not _returnvalue)
        (`TimelineComponent.PlayFromStart` (`self.FadePPSaturation`)))
      (`TimelineComponent.ReverseFromEnd` _fadeppdirection)))
  (set `self.CurrentChoiceIndex` SelectedChoiceIndex)
  (bind _foundwidgets (`WidgetBlueprintLibrary.GetAllWidgetsOfClass` "/Game/StoryFramework/Core/UserInterface/Widgets/StoryChoice_W.StoryChoice_W_C"))
  (`/Game/StoryFramework/Core/UserInterface/Widgets/StoryChoice_W.UpdateChoice` (`|GetArrayItem` _foundwidgets) (`self.CurrentChoiceIndex`)))

(fn `UserConstructionScript`)