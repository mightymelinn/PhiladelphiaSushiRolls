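; Blueprint function library of general camera helpers for the Story Framework (SF).
; It reports player 0's view target and whether it is the pawn, fetches an SFDefaultCamera_CC from the player character by index, and converts seconds into a play rate.
; Fades run either through the camera manager or through a WidgetFade_W overlay, which replaces the first existing top-level fade widget before starting.
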(fn `FadeCamera`
  (params (FromAlpha :type "Float (single-precision)") (ToAlpha :type "Float (single-precision)") (Duration :type "Float (single-precision)") (Color :type "LinearColor Structure") (bShouldFadeAudio :type Boolean) (bHoldWhenFinished :type Boolean))
  (`PlayerCameraManager.StartCameraFade` (`GameplayStatics.GetPlayerCameraManager` null) FromAlpha ToAlpha Duration Color bShouldFadeAudio bHoldWhenFinished))

(fn `GetControllerViewTarget`
  (returns (ReturnValue :type "Actor Object Reference") (IsViewTargetPlayer :type Boolean))
  (bind _returnvalue (`GameplayStatics.GetPlayerController` null))
  (bind _returnvalue_2 (`Controller.GetViewTarget` _returnvalue))
  (`/Engine/EditorBlueprintResources/StandardMacros.IsValid` _returnvalue
    (:`Is Valid`
      (return _returnvalue_2 (== _returnvalue_2 (`GameplayStatics.GetPlayerPawn` null))))))

(fn `GetPlayRateLengthInSeconds`
  (params (`Length(InSec)` :type "Float (double-precision)"))
  (returns (`Length(Rate)` :type "Float (double-precision)"))
  (return (/ 1.0 `Length(InSec)`)))

(fn `GetSFCameraComponentFromCharacter`
  (params (ComponentIndex :type Integer :default 0))
  (returns (Reference :type "/Game/StoryFramework/Core/Blueprints/Components/Other/SFDefaultCamera_CC Object Reference"))
  (bind _returnvalue (`GameplayStatics.GetPlayerCharacter` null))
  (bind _output (`|GetArrayItem` (`Actor.K2_GetComponentsByClass` _returnvalue "/Game/StoryFramework/Core/Blueprints/Components/Other/SFDefaultCamera_CC.SFDefaultCamera_CC_C") ComponentIndex))
  (`/Engine/EditorBlueprintResources/StandardMacros.IsValid` _returnvalue
    (:`Is Valid`
      (`/Engine/EditorBlueprintResources/StandardMacros.IsValid` _output
        (:`Is Valid`
          (return _output))))))

(fn `WidgetFadeCamera`
  (params (FadeDirection :type Integer) (`FadeSpeed (InSec)` :type "Float (double-precision)") (ZOrder :type Integer :default 2))
  (locals (WidgetFadeRef :type "/Game/StoryFramework/Core/UserInterface/Widgets/WidgetFade_W Object Reference") (FadeDirRef :type Integer) (FadeSpeedRef :type "Float (double-precision)"))
  (bind _widgetfaderef (`local.WidgetFadeRef`))
  (set `local.FadeDirRef` FadeDirection)
  (set `local.FadeSpeedRef` `FadeSpeed (InSec)`)
  (bind _foundwidgets (`WidgetBlueprintLibrary.GetAllWidgetsOfClass` null "/Game/StoryFramework/Core/UserInterface/Widgets/WidgetFade_W.WidgetFade_W_C"))
  (if (`KismetArrayLibrary.Array_IsValidIndex` _foundwidgets)
    (`Widget.RemoveFromParent` (`|GetArrayItem` _foundwidgets)))
  (bind _returnvalue (`|CreateWidget` "/Game/StoryFramework/Core/UserInterface/Widgets/WidgetFade_W.WidgetFade_W_C"))
  (set `local.WidgetFadeRef` _returnvalue)
  (set `/Game/StoryFramework/Core/UserInterface/Widgets/WidgetFade_W.FadeDirection` (`local.FadeDirRef`) _widgetfaderef)
  (set `/Game/StoryFramework/Core/UserInterface/Widgets/WidgetFade_W.FadeSpeed(InSec)` (`local.FadeSpeedRef`) _widgetfaderef)
  (`/Game/StoryFramework/Core/UserInterface/Widgets/WidgetFade_W.StartFade` _widgetfaderef)
  (`UserWidget.AddToViewport` (`local.WidgetFadeRef`) ZOrder))