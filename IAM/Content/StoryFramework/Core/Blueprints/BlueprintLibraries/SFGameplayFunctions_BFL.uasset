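; Blueprint function library of StoryFramework gameplay helpers shared across interaction, dialogue, sequences, menus, saving, audio and UI.
; Getters fetch the framework's manager components from player controller 0 through an interface message, and most other helpers build on them.
; Save helpers record destroyed, spawned, interacted and tagged actors in the SaveManager, mostly per level.
; Menu helpers swap input modes and Enhanced Input contexts, while outlines toggle custom depth on mesh components.
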(fn `AddInteractActors (SaveGame)`
  (params (InteractActor :type "/Game/StoryFramework/Core/Blueprints/InteractableBase_BP Object Reference") (DataString :type String))
  (locals (FindInteractActorNames :type "Array of String") (TargetInteractActor :type "/Game/StoryFramework/Core/Blueprints/InteractableBase_BP Object Reference") (TargetInteractDataString :type String) (TempInteractedActors :type "Map of String to String"))
  (set `local.TargetInteractActor` InteractActor)
  (set `local.TargetInteractDataString` DataString)
  (bind _returnvalue (`GameplayStatics.GetCurrentLevelName` null))
  (bind (_value _returnvalue_2) (`BlueprintMapLibrary.Map_Find` (`/Game/StoryFramework/SaveGame/Blueprints/SFSaveManager_AC.InteractActors` (`self.GetSFSaveManager (Controller)` null)) (`KismetStringLibrary.Conv_StringToName` _returnvalue)))
  (if _returnvalue_2
    (set `local.TempInteractedActors` (`.InteractActors_4_C8B2A9F140091C23CC881D940E84A020` (break `/Game/StoryFramework/SaveGame/Blueprints/Structures/LevelInteractSaveData_S` _value))))
  (`BlueprintMapLibrary.Map_Add` (`local.TempInteractedActors`) (`KismetSystemLibrary.GetObjectName` (`local.TargetInteractActor`)) (`local.TargetInteractDataString`))
  (`BlueprintMapLibrary.Map_Add` (`/Game/StoryFramework/SaveGame/Blueprints/SFSaveManager_AC.InteractActors` (`self.GetSFSaveManager (Controller)` null)) (`KismetStringLibrary.Conv_StringToName` _returnvalue) (make `/Game/StoryFramework/SaveGame/Blueprints/Structures/LevelInteractSaveData_S` (`local.TempInteractedActors`))))

(fn `AddPlayerConTag (Controller)`
  (params (NewTag :type Name))
  (`KismetArrayLibrary.Array_Add` (`/Game/StoryFramework/Core/Blueprints/Components/Core/SFInteractionManager_AC.ConsequentialTags` (`self.GetSFInteractionManager (Controller)` null)) NewTag)
  (return))

(fn `Close SFMenu`
  (params (WidgetClass :type "UserWidget Class Reference"))
  (bind _interactionmanager (`self.GetSFInteractionManager (Controller)` null))
  (bind _returnvalue (`GameplayStatics.GetPlayerController` null))
  (bind _foundwidgets (`WidgetBlueprintLibrary.GetAllWidgetsOfClass` null WidgetClass))
  (for _array_element _foundwidgets
    (`Widget.RemoveFromParent` _array_element))
  (set `PlayerController.bShowMouseCursor` false _returnvalue)
  (`WidgetBlueprintLibrary.SetInputMode_GameOnly` _returnvalue true)
  (set `/Game/StoryFramework/Core/SFGameInstance_BP.CurrentSFMenu` null (`self.GetSFGameInstance` null))
  (`/Engine/EditorBlueprintResources/StandardMacros.IsValid` _interactionmanager
    (:`Is Valid`
      (`self.UpdateInputMappingContext` (`/Game/StoryFramework/Core/Blueprints/Components/Core/SFInteractionManager_AC.CurrentInputMappingContext` _interactionmanager)))))

(fn `Create SFMenu`
  (params (WidgetClass :type "UserWidget Class Reference") (ZOrder :type Integer :default 0))
  (returns (ReturnValue :type "UserWidget Object Reference"))
  (bind _returnvalue (`GameplayStatics.GetPlayerController` null))
  (bind _returnvalue_2 (`|CreateWidget` WidgetClass))
  (bind _output_get (set `/Game/StoryFramework/Core/SFGameInstance_BP.CurrentSFMenu` (cast `/Game/StoryFramework/Menus/UserInterface/MenuMaster_W` _returnvalue_2 :!pure true) (`self.GetSFGameInstance` null)))
  (`UserWidget.AddToViewport` _output_get ZOrder)
  (set `PlayerController.bShowMouseCursor` true _returnvalue)
  (`WidgetBlueprintLibrary.SetInputMode_GameAndUIEx` _returnvalue _returnvalue_2 "DoNotLock" false true)
  (`self.UpdateInputMappingContext` "/Game/StoryFramework/Menus/Input/WidgetMenu_IMC.WidgetMenu_IMC" false)
  (return _returnvalue_2))

(fn `CreateCustomPopup`
  (params (Header :type Text) (Description :type Text) (Image :type "Texture2D Object Reference") (Duration :type "Float (single-precision)" :default 5.0) (DisplayUMCPrompt :type Boolean))
  (returns (ReturnValue :type "/Game/StoryFramework/Core/UserInterface/Widgets/PopupMaster_W Object Reference"))
  (bind _returnvalue (`|CreateWidget` "/Game/StoryFramework/Core/UserInterface/Widgets/PopupMaster_W.PopupMaster_W_C"))
  (`/Game/StoryFramework/Core/UserInterface/Widgets/PopupMaster_W.ShowCustomPopup` _returnvalue Header Description Image Duration DisplayUMCPrompt)
  (`UserWidget.AddToViewport` _returnvalue 0)
  (return _returnvalue))

(fn `DestroyActor (SaveGame)`
  (params (Target :type "Actor Object Reference"))
  (locals (CheckInteractionData :type "Array of /Game/StoryFramework/Core/Blueprints/Structures/InteractableData_S Structure") (TempDestroyedActors :type "Array of String"))
  (bind _returnvalue (`GameplayStatics.GetCurrentLevelName` null))
  (bind (_value _returnvalue_2) (`BlueprintMapLibrary.Map_Find` (`/Game/StoryFramework/SaveGame/Blueprints/SFSaveManager_AC.DestroyedActors` (`self.GetSFSaveManager (Controller)` null)) (`KismetStringLibrary.Conv_StringToName` _returnvalue)))
  (if _returnvalue_2
    (set `local.TempDestroyedActors` (`.DestroyedActors_3_E306C5D04125EAE0A15D14A63A103B54` (break `/Game/StoryFramework/SaveGame/Blueprints/Structures/LevelDestroyedSaveData_S` _value))))
  (`KismetArrayLibrary.Array_Add` (`local.TempDestroyedActors`) (`KismetSystemLibrary.GetObjectName` Target))
  (`BlueprintMapLibrary.Map_Add` (`/Game/StoryFramework/SaveGame/Blueprints/SFSaveManager_AC.DestroyedActors` (`self.GetSFSaveManager (Controller)` null)) (`KismetStringLibrary.Conv_StringToName` _returnvalue) (make `/Game/StoryFramework/SaveGame/Blueprints/Structures/LevelDestroyedSaveData_S` (`local.TempDestroyedActors`)))
  (`Actor.K2_DestroyActor` Target))

(fn `FindInputInInputMappingDataTable`
  (params (InputKey :type "Key Structure" :default "None"))
  (returns (FoundKeySettings :type "/Game/StoryFramework/Core/Blueprints/Structures/InputMap_S Structure"))
  (locals (TargetKeySettings :type "/Game/StoryFramework/Core/Blueprints/Structures/InputMap_S Structure"))
  (bind _outrownames (`DataTableFunctionLibrary.GetDataTableRowNames` "/Game/StoryFramework/Core/Blueprints/DataTables/InputMap_DT.InputMap_DT"))
  (for _array_element _outrownames
    (bind _returnvalue (`|GetDataTableRow` "/Game/StoryFramework/Core/Blueprints/DataTables/InputMap_DT.InputMap_DT" _array_element)
      (:`then`
        (if (== (`.TargetKey_25_4E590A864CC130D220975F8DDBC784CE` (break `/Game/StoryFramework/Core/Blueprints/Structures/InputMap_S` _returnvalue)) InputKey)
          (set `local.TargetKeySettings` _returnvalue)
          (break)))))
  (return (`local.TargetKeySettings`)))

(fn `GetCurrentSFV (Instance)`
  (returns (StoryFrameworkValues :type "/Game/StoryFramework/Core/Blueprints/DataAssets/SFCustomization_PDA Object Reference"))
  (bind _returnvalue (`self.GetSFGameInstance` null))
  (`/Engine/EditorBlueprintResources/StandardMacros.IsValid` _returnvalue
    (:`Is Valid`
      (return (`/Game/StoryFramework/Core/SFGameInstance_BP.SFCustomizationAsset` _returnvalue)))))

(fn `GetDialogueGraphReference`
  (returns (DialogueGraph :type "/Game/StoryFramework/Core/Dialogue/DialogueGraphActor Object Reference"))
  (bind _outactors (`GameplayStatics.GetAllActorsWithTag` null "SFDialogueGraph"))
  (return (cast `/Game/StoryFramework/Core/Dialogue/DialogueGraphActor` (`|GetArrayItem` _outactors) :!pure true)))

(fn `GetPauseMenuWidget (Reference)`
  (returns (MenuWidget :type "/Game/StoryFramework/Menus/UserInterface/PauseMenu_W Object Reference"))
  (bind _foundwidgets (`WidgetBlueprintLibrary.GetAllWidgetsOfClass` null "/Game/StoryFramework/Menus/UserInterface/PauseMenu_W.PauseMenu_W_C"))
  (if (`KismetArrayLibrary.Array_IsNotEmpty` _foundwidgets)
    (return (`|GetArrayItem` _foundwidgets))
    (else
      (return null))))

(fn `GetPlayerConTags (Controller)`
  (returns (ConTags :type "Array of Name"))
  (bind _interactionmanager (message `/Game/StoryFramework/Core/Blueprints/BlueprintInterfaces/SFPlayerControllerData_BPI.GetSFComponents` (`GameplayStatics.GetPlayerController` null)))
  (return (`/Game/StoryFramework/Core/Blueprints/Components/Core/SFInteractionManager_AC.ConsequentialTags` _interactionmanager)))

(fn `GetSFCameraManager (Controller)`
  (returns (CameraManager :type "/Game/StoryFramework/Core/Blueprints/Components/Core/SFCameraManager_AC Object Reference"))
  (bind (_interactionmanager _inventorymanager _sequencemanager _cameramanager) (message `/Game/StoryFramework/Core/Blueprints/BlueprintInterfaces/SFPlayerControllerData_BPI.GetSFComponents` (`GameplayStatics.GetPlayerController` null)))
  (return _cameramanager))

(fn `GetSFGameInstance`
  (returns (ReturnValue :type "/Game/StoryFramework/Core/SFGameInstance_BP Object Reference"))
  (bind _sfgameinstance (message `/Game/StoryFramework/Core/Blueprints/BlueprintInterfaces/SFGameInstance_BP.GetSFGameInstance` (`GameplayStatics.GetGameInstance` null)))
  (return _sfgameinstance))

(fn `GetSFInteractionManager (Controller)`
  (returns (InteractionManager :type "/Game/StoryFramework/Core/Blueprints/Components/Core/SFInteractionManager_AC Object Reference"))
  (bind _interactionmanager (message `/Game/StoryFramework/Core/Blueprints/BlueprintInterfaces/SFPlayerControllerData_BPI.GetSFComponents` (`GameplayStatics.GetPlayerController` null)))
  (return _interactionmanager))

(fn `GetSFInventoryManager (Controller)`
  (returns (InventoryManager :type "/Game/StoryFramework/Core/Blueprints/Components/Core/SFInventoryManager_AC Object Reference"))
  (bind (_interactionmanager _inventorymanager) (message `/Game/StoryFramework/Core/Blueprints/BlueprintInterfaces/SFPlayerControllerData_BPI.GetSFComponents` (`GameplayStatics.GetPlayerController` null)))
  (return _inventorymanager))

(fn `GetSFSaveManager (Controller)`
  (returns (SaveManager :type "/Game/StoryFramework/SaveGame/Blueprints/SFSaveManager_AC Object Reference"))
  (bind (_interactionmanager _inventorymanager _sequencemanager _cameramanager _savemanager) (message `/Game/StoryFramework/Core/Blueprints/BlueprintInterfaces/SFPlayerControllerData_BPI.GetSFComponents` (`GameplayStatics.GetPlayerController` null)))
  (return _savemanager))

(fn `GetSFSequenceManager (Controller)`
  (returns (SequenceManager :type "/Game/StoryFramework/Core/Blueprints/Components/Core/SFSequenceManager_AC Object Reference"))
  (bind (_interactionmanager _inventorymanager _sequencemanager) (message `/Game/StoryFramework/Core/Blueprints/BlueprintInterfaces/SFPlayerControllerData_BPI.GetSFComponents` (`GameplayStatics.GetPlayerController` null)))
  (return _sequencemanager))

(fn `GetTargetNPCByID`
  (params (ID :type Name))
  (returns (FoundNPC :type "Actor Object Reference"))
  (locals (FoundNPCTarget :type "Actor Object Reference"))
  (bind _outactors (`GameplayStatics.GetAllActorsWithInterface` null "/Game/StoryFramework/Core/Blueprints/BlueprintInterfaces/DialogueInfo_BPI.DialogueInfo_BPI_C"))
  (for _array_element _outactors
    (bind _npcinfo (message `/Game/StoryFramework/Core/Blueprints/BlueprintInterfaces/DialogueInfo_BPI.GetOwnerDialogueData` _array_element))
    (if (== (`.ID_11_C426EBEC4AFCAFAF6BC5499A79B1EF4C` (break `/Game/StoryFramework/Core/Blueprints/Structures/NPCBIName_S` (`.NameInfo_15_5EBED67B48685247F75CBE8C29A24478` (break `/Game/StoryFramework/Core/Blueprints/Structures/NPCBasicInfo_S` _npcinfo)))) ID)
      (set `local.FoundNPCTarget` _array_element)
      (break)))
  (return (`local.FoundNPCTarget`)))

(fn `IsUsingGamepad`
  (returns (ReturnValue :type Boolean))
  (bind _interactionmanager (message `/Game/StoryFramework/Core/Blueprints/BlueprintInterfaces/SFPlayerControllerData_BPI.GetSFComponents` (`GameplayStatics.GetPlayerController` null)))
  (`/Engine/EditorBlueprintResources/StandardMacros.IsValid` _interactionmanager
    (:`Is Valid`
      (return (`/Game/StoryFramework/Core/Blueprints/Components/Core/SFInteractionManager_AC.IsUsingGamepad` _interactionmanager)))))

(fn `LoadSystemInfo (SaveGame)`
  (returns (SystemData :type "/Game/StoryFramework/SaveGame/Blueprints/Structures/SystemSaveData_S Structure"))
  (bind _returnvalue (`GameplayStatics.LoadGameFromSlot` "SFSaveSlot"))
  (bind _assfsave_game_bp (cast `/Game/StoryFramework/SaveGame/SFSaveGame_BP` _returnvalue))
  (return (`/Game/StoryFramework/SaveGame/SFSaveGame_BP.SystemData` _assfsave_game_bp)))

(fn `OpenLevel (SaveGame)`
  (params (LevelName :type Name) (IgnorePlayerLocation :type Boolean))
  (`/Game/StoryFramework/Core/SFGameInstance_BP.OpenLevelSave` (cast `/Game/StoryFramework/Core/SFGameInstance_BP` (`GameplayStatics.GetGameInstance` null) :!pure true) LevelName IgnorePlayerLocation))

(fn `OutlineActor (PostProcess)`
  (params (Actor :type "Actor Object Reference") (Remove :type Boolean))
  (bind _returnvalue (`Actor.K2_GetComponentsByClass` Actor "/Script/Engine.SkeletalMeshComponent"))
  (bind _returnvalue_2 (`Actor.K2_GetComponentsByClass` Actor "/Script/Engine.StaticMeshComponent"))
  (`/Engine/EditorBlueprintResources/StandardMacros.IsValid` Actor
    (:`Is Valid`
      (if (and (>= (`KismetArrayLibrary.Array_LastIndex` _returnvalue_2) 0) (not (`Actor.ActorHasTag` Actor "IgnoreOutlines")))
        (for _array_element _returnvalue_2
          (if (not (`ActorComponent.ComponentHasTag` _array_element "IgnoreOutlines"))
            (`PrimitiveComponent.SetRenderCustomDepth` _array_element (not Remove)))))
      (if (>= (`KismetArrayLibrary.Array_LastIndex` _returnvalue) 0)
        (for _array_element_2 _returnvalue
          (if (not (`ActorComponent.ComponentHasTag` _array_element_2 "IgnoreOutlines"))
            (`PrimitiveComponent.SetRenderCustomDepth` _array_element_2 (not Remove))))))))

(fn `PlayerHasConTag (Controller)`
  (params (Find :type Name))
  (returns (Found :type Boolean) (Priority :type Integer))
  (bind _interactionmanager (message `/Game/StoryFramework/Core/Blueprints/BlueprintInterfaces/SFPlayerControllerData_BPI.GetSFComponents` (`GameplayStatics.GetPlayerController` null)))
  (bind _consequentialtags (`/Game/StoryFramework/Core/Blueprints/Components/Core/SFInteractionManager_AC.ConsequentialTags` _interactionmanager))
  (return (`KismetArrayLibrary.Array_Contains` _consequentialtags Find) (`KismetArrayLibrary.Array_Find` _consequentialtags Find)))

(fn `PlaySound2D FromSFV`
  (params (SoundName :type String) (FallbackSound :type "/Game/StoryFramework/Core/Blueprints/Structures/EditableSoundTemplate_S Structure"))
  (bind (_sound _volumemulti _pitchmulti) (break `/Game/StoryFramework/Core/Blueprints/Structures/EditableSoundTemplate_S` FallbackSound))
  (bind _value (`BlueprintMapLibrary.Map_Find` (`/Game/StoryFramework/Core/Blueprints/DataAssets/SFCustomization_PDA.ListOfSounds` (`self.GetCurrentSFV (Instance)` null)) SoundName))
  (`/Engine/EditorBlueprintResources/StandardMacros.IsValid` (`self.GetSFInteractionManager (Controller)` null)
    (:`Is Valid`
      (`GameplayStatics.PlaySound2D` null (break `/Game/StoryFramework/Core/Blueprints/Structures/EditableSoundTemplate_S` _value) (`.VolumeMulti_5_2D74A3644EF27AEF293B5C86F9E62B19` (break `/Game/StoryFramework/Core/Blueprints/Structures/EditableSoundTemplate_S` _value)) (`.PitchMulti_7_45FBD7014241F750DF880DB6EB1473C7` (break `/Game/StoryFramework/Core/Blueprints/Structures/EditableSoundTemplate_S` _value)) 0.0 null null))
    (:`Is Not Valid`
      (`GameplayStatics.PlaySound2D` null _sound _volumemulti _pitchmulti 0.0 null null)))
  (return))

(fn `PlaySound3D FromSFV`
  (params (SoundName :type String) (Location :type "Vector Structure") (FallbackSound :type "/Game/StoryFramework/Core/Blueprints/Structures/EditableSoundTemplate_S Structure"))
  (bind (_sound _volumemulti _pitchmulti) (break `/Game/StoryFramework/Core/Blueprints/Structures/EditableSoundTemplate_S` FallbackSound))
  (bind _value (`BlueprintMapLibrary.Map_Find` (`/Game/StoryFramework/Core/Blueprints/DataAssets/SFCustomization_PDA.ListOfSounds` (`self.GetCurrentSFV (Instance)` null)) SoundName))
  (`/Engine/EditorBlueprintResources/StandardMacros.IsValid` (`self.GetSFInteractionManager (Controller)` null)
    (:`Is Valid`
      (`GameplayStatics.PlaySoundAtLocation` null (break `/Game/StoryFramework/Core/Blueprints/Structures/EditableSoundTemplate_S` _value) Location (struct) (`.VolumeMulti_5_2D74A3644EF27AEF293B5C86F9E62B19` (break `/Game/StoryFramework/Core/Blueprints/Structures/EditableSoundTemplate_S` _value)) (`.PitchMulti_7_45FBD7014241F750DF880DB6EB1473C7` (break `/Game/StoryFramework/Core/Blueprints/Structures/EditableSoundTemplate_S` _value)) 0.0 null null null null))
    (:`Is Not Valid`
      (`GameplayStatics.PlaySoundAtLocation` null _sound Location (struct) _volumemulti _pitchmulti 0.0 null null null null)))
  (return))

(fn `RemovePlayerConTag (Controller)`
  (params (RemoveTag :type Name))
  (`KismetArrayLibrary.Array_RemoveItem` (`/Game/StoryFramework/Core/Blueprints/Components/Core/SFInteractionManager_AC.ConsequentialTags` (`self.GetSFInteractionManager (Controller)` null)) RemoveTag)
  (return))

(fn `ResetSFCameraEvents (CamComponent)`
  (`/Game/StoryFramework/Core/Blueprints/Components/Other/SFDefaultCamera_CC.ResetAllCameraEvents` (`/Game/StoryFramework/Core/Blueprints/BlueprintLibraries/SFCameraGeneralFunctions_BFL.GetSFCameraComponentFromCharacter` 0))
  (return))

(fn `SaveActorTags (SaveGame)`
  (params (Actor :type "Actor Object Reference") (Tags :type "Array of Name"))
  (locals (DoesActorExist :type Boolean) (ExistingActorIndex :type Integer) (LevelActorTagSave :type "/Game/StoryFramework/SaveGame/Blueprints/Structures/LevelActorTagSave_S Structure"))
  (bind _levelactortagsave (`local.LevelActorTagSave`))
  (bind _actortags (`/Game/StoryFramework/SaveGame/Blueprints/SFSaveManager_AC.ActorTags` (`self.GetSFSaveManager (Controller)` null)))
  (bind _output_get (set `local.LevelActorTagSave` (make `/Game/StoryFramework/SaveGame/Blueprints/Structures/LevelActorTagSave_S` (`KismetSystemLibrary.GetObjectName` Actor) Tags)))
  (for (_array_element _array_index) (`/Game/StoryFramework/SaveGame/Blueprints/SFSaveManager_AC.ActorTags` (`self.GetSFSaveManager (Controller)` null))
    (if (`KismetStringLibrary.EqualEqual_StrStr` (`.ActorName_8_79E4D9E84CD5CE2B83A07FAD9870FD1B` (break `/Game/StoryFramework/SaveGame/Blueprints/Structures/LevelActorTagSave_S` _array_element)) (`.ActorName_8_79E4D9E84CD5CE2B83A07FAD9870FD1B` (break `/Game/StoryFramework/SaveGame/Blueprints/Structures/LevelActorTagSave_S` _output_get)))
      (set `local.DoesActorExist` true)
      (set `local.ExistingActorIndex` _array_index)
      (break)))
  (if (`local.DoesActorExist`)
    (`KismetArrayLibrary.Array_Set` _actortags (`local.ExistingActorIndex`) _levelactortagsave)
    (else
      (`KismetArrayLibrary.Array_Add` _actortags _levelactortagsave))))

(fn `SaveSpawnedActor (SaveGame)`
  (params (Target :type "Actor Object Reference (by ref)") (`Interactable Data` :type "/Game/StoryFramework/Core/Blueprints/Structures/InteractableData_S Structure") (StaticMeshActor :type "StaticMesh Object Reference"))
  (bind _savemanager (`self.GetSFSaveManager (Controller)` null))
  (bind _returnvalue (`GameplayStatics.GetCurrentLevelName` null))
  (bind _returnvalue_2 (`KismetStringLibrary.Conv_StringToName` _returnvalue))
  (`KismetArrayLibrary.Array_Add` (`/Game/StoryFramework/SaveGame/Blueprints/SFSaveManager_AC.SpawnedActors` _savemanager) (make `/Game/StoryFramework/SaveGame/Blueprints/Structures/LevelActorSaveData_S` _returnvalue_2 (`GameplayStatics.GetObjectClass` Target) (`Actor.GetTransform` Target) (`Actor.Tags` Target) `Interactable Data` StaticMeshActor))
  (bind _destroyedactors (break `/Game/StoryFramework/SaveGame/Blueprints/Structures/LevelDestroyedSaveData_S` (`BlueprintMapLibrary.Map_Find` (`/Game/StoryFramework/SaveGame/Blueprints/SFSaveManager_AC.DestroyedActors` _savemanager) _returnvalue_2)))
  (bind _returnvalue_3 (`KismetArrayLibrary.Array_Find` _destroyedactors (`KismetSystemLibrary.GetDisplayName` Target)))
  (if (> _returnvalue_3 -1)
    (`KismetArrayLibrary.Array_RemoveItem` _destroyedactors (`|GetArrayItem` _destroyedactors _returnvalue_3))))

(fn `SFMovementCondition`
  (params (IgnorePerformActionCheck :type Boolean))
  (returns (ReturnValue :type Boolean))
  (bind _interactionmanager (`self.GetSFInteractionManager (Controller)` null))
  (bind _interactionmanager_2 (`self.GetSFInteractionManager (Controller)` null))
  (if (and (`/Game/StoryFramework/Core/Blueprints/Components/Core/SFInteractionManager_AC.IsInDialogWithNPC` _interactionmanager) (`KismetSystemLibrary.IsValid` (`/Game/StoryFramework/Core/Blueprints/Components/Core/SFInteractionManager_AC.TargetNPCActor` _interactionmanager)))
    (bind _npcinfo (message `/Game/StoryFramework/Core/Blueprints/BlueprintInterfaces/DialogueInfo_BPI.GetOwnerDialogueData` (`/Game/StoryFramework/Core/Blueprints/Components/Core/SFInteractionManager_AC.TargetNPCActor` (`self.GetSFInteractionManager (Controller)` null))))
    (if (`|EnumInequality` (`.CameraEffect_6_799D78A04BB219493E77BFAEE2CF2590` (break `/Game/StoryFramework/Core/Blueprints/Structures/NPCBIOther_S` (`.Other_18_9B43471A480BF2DFBA4E079F194A91BF` (break `/Game/StoryFramework/Core/Blueprints/Structures/NPCBasicInfo_S` _npcinfo)))) "NewEnumerator2")
      (return false)
      (else
        (return true)))
    (elif (`Actor.ActorHasTag` (`Controller.GetViewTarget` (`GameplayStatics.GetPlayerController` null)) "CustomViewInteraction")
      (return false)
      (elif IgnorePerformActionCheck
        (return true)
        (else
          (return (not (and (`/Game/StoryFramework/Core/Blueprints/Components/Core/SFInteractionManager_AC.IsPerfomingAction` _interactionmanager_2) (`|EnumEquality` (`/Game/StoryFramework/Core/Blueprints/Components/Core/SFInteractionManager_AC.ActionRestrictions` _interactionmanager_2) "NewEnumerator1")))))))))

(fn `SimpleFirstPersonComponentHide`
  (params (Target :type "SceneComponent Object Reference"))
  (`SceneComponent.SetVisibility` Target (select `bool` (`/Game/StoryFramework/Core/Blueprints/Components/Core/SFSequenceManager_AC.IsCurrentSequencePlaying` (`self.GetSFSequenceManager (Controller)` null)) :`false` (select `/Game/StoryFramework/Core/Blueprints/Enumerators/CameraPresets_E` (`/Game/StoryFramework/Core/Blueprints/Components/Other/SFDefaultCamera_CC.CurrentCameraPreset` (`/Game/StoryFramework/Core/Blueprints/BlueprintLibraries/SFCameraGeneralFunctions_BFL.GetSFCameraComponentFromCharacter` 0)) :`NewEnumerator3` true) :`true` true) false))

(fn `ToggleCinemaCrop`
  (params (VerticalCropSize :type Integer))
  (returns (ToggledOnWidgetRef :type "/Game/StoryFramework/Core/UserInterface/Widgets/CinemaCrop_W Object Reference"))
  (bind _foundwidgets (`WidgetBlueprintLibrary.GetAllWidgetsOfClass` null "/Game/StoryFramework/Core/UserInterface/Widgets/CinemaCrop_W.CinemaCrop_W_C"))
  (if (`KismetArrayLibrary.Array_IsEmpty` _foundwidgets)
    (bind _returnvalue (`|CreateWidget` "/Game/StoryFramework/Core/UserInterface/Widgets/CinemaCrop_W.CinemaCrop_W_C"))
    (`/Game/StoryFramework/Core/UserInterface/Widgets/CinemaCrop_W.Initialize` _returnvalue VerticalCropSize)
    (bind _foundwidgets_2 (`WidgetBlueprintLibrary.GetAllWidgetsOfClass` null "/Game/StoryFramework/Core/UserInterface/Widgets/InSequence_W.InSequence_W_C"))
    (if (`KismetArrayLibrary.Array_IsNotEmpty` _foundwidgets_2)
      (`/Game/StoryFramework/Core/UserInterface/Widgets/InSequence_W.UpdateSubtitleOffset` (`|GetArrayItem` _foundwidgets_2) VerticalCropSize))
    (return _returnvalue)
    (else
      (`Widget.RemoveFromParent` (`|GetArrayItem` _foundwidgets)))))

(fn `TogglePauseGame (Widget)`
  (params (PauseWidgetClass :type "UserWidget Class Reference") (UseWidgetNavInputMapping :type Boolean))
  (locals (TargetMappingContext :type "InputMappingContext Object Reference") (TargetUseWidgetNav :type Boolean))
  (bind _sequencemanager (`self.GetSFSequenceManager (Controller)` null))
  (bind _sequencemanager_2 (`self.GetSFSequenceManager (Controller)` null))
  (bind _currentsubtitledsound (`/Game/StoryFramework/Core/Blueprints/Components/Core/SFSequenceManager_AC.CurrentSubtitledSound` _sequencemanager))
  (set `local.TargetUseWidgetNav` UseWidgetNavInputMapping)
  (bind _foundwidgets (`WidgetBlueprintLibrary.GetAllWidgetsOfClass` null PauseWidgetClass))
  (if (`KismetArrayLibrary.Array_IsNotEmpty` _foundwidgets)
    (bind _aspause_menu_w (cast `/Game/StoryFramework/Menus/UserInterface/PauseMenu_W` (`|GetArrayItem` _foundwidgets) :!pure true))
    (if (`/Game/StoryFramework/Menus/UserInterface/PauseMenu_W.IsInSettings` _aspause_menu_w)
      (`/Game/StoryFramework/Menus/UserInterface/PauseMenu_W.OnCloseButtonPressed` _aspause_menu_w)
      (else
        (`self.Close SFMenu` PauseWidgetClass)
        (`GameplayStatics.SetGamePaused` null)
        (`/Engine/EditorBlueprintResources/StandardMacros.IsValid` _currentsubtitledsound
          (:`Is Valid`
            (`AudioComponent.SetPaused` _currentsubtitledsound false)
            (`/Game/StoryFramework/Core/UserInterface/Widgets/InSequence_W.OnPause` (`/Game/StoryFramework/Core/Blueprints/Components/Core/SFSequenceManager_AC.InSequenceWidgetRef` _sequencemanager) true)))))
    (else
      (`self.Create SFMenu` PauseWidgetClass 10)
      (`GameplayStatics.SetGamePaused` null true)
      (if (`/Game/StoryFramework/Core/Blueprints/Components/Core/SFSequenceManager_AC.IsSubtitledSoundPlaying` _sequencemanager_2)
        (`AudioComponent.SetPaused` (`/Game/StoryFramework/Core/Blueprints/Components/Core/SFSequenceManager_AC.CurrentSubtitledSound` _sequencemanager_2) true)
        (`/Game/StoryFramework/Core/UserInterface/Widgets/InSequence_W.OnPause` (`/Game/StoryFramework/Core/Blueprints/Components/Core/SFSequenceManager_AC.InSequenceWidgetRef` _sequencemanager_2) false)))))

(fn `UpdateInputMappingContext`
  (params (NewMappingContext :type "InputMappingContext Object Reference") (UpdateInteractionVariable :type Boolean :default true))
  (bind _interactionmanager (`self.GetSFInteractionManager (Controller)` null))
  (bind _returnvalue (pcsubsystem `EnhancedInputLocalPlayerSubsystem` (`GameplayStatics.GetPlayerController` null)))
  (`EnhancedInputSubsystemInterface.ClearAllMappings` _returnvalue)
  (`EnhancedInputSubsystemInterface.AddMappingContext` _returnvalue NewMappingContext 0 (make `ModifyContextOptions` true))
  (if UpdateInteractionVariable
    (`/Engine/EditorBlueprintResources/StandardMacros.IsValid` _interactionmanager
      (:`Is Valid`
        (set `/Game/StoryFramework/Core/Blueprints/Components/Core/SFInteractionManager_AC.CurrentInputMappingContext` NewMappingContext _interactionmanager)))))