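; Player camera manager for the story framework that turns the player's view toward a target over a given number of seconds, via the LookatTarget interface event.
; The event stores the current camera rotation, then restarts a timeline with an ease-out curve and a play rate derived from the duration.
; Timeline updates are written to set control rotation from a shortest-path lerp toward the look-at rotation, keeping roll at zero.
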(event `/Game/StoryFramework/Core/Blueprints/BlueprintInterfaces/SFPlayerCameraManager_BPI.LookAtTarget`
  (params (Target :type "Vector Structure") (`Speed(InSec)` :type "Float (double-precision)"))
  ;[0.04314 0.04314 0.05098] Blueprint Interface Events
  (set `self.PreviousCameraRotation` (`self.GetCameraRotation`))
  (`self.UpdateTargetTimelineAndPlay` (`self.LookAtTargetTimeline`) (`/Game/StoryFramework/Core/Blueprints/BlueprintLibraries/SFCameraGeneralFunctions_BFL.GetPlayRateLengthInSeconds` `Speed(InSec)`)))

(fn `UpdateTargetTimelineAndPlay`
  (params (`Target Timeline` :type "TimelineComponent Object Reference") (NewPlayRate :type "Float (double-precision)"))
  (`TimelineComponent.SetPlayRate` `Target Timeline` NewPlayRate)
  (`TimelineComponent.SetFloatCurve` `Target Timeline` "/Game/StoryFramework/Core/Blueprints/Curves/EaseOut_FloatCurve.EaseOut_FloatCurve" "Alpha")
  (`TimelineComponent.PlayFromStart` `Target Timeline`)
  (return))

(fn `UserConstructionScript`)