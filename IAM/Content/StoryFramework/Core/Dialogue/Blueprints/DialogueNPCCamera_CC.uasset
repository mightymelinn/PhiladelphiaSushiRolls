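; Dialogue NPC camera component that plays a simple continuous zoom-in or directional pan while possessed.
; On possession, a looping timer set to the current frame delta calls PlayAnimations, nudging FOV or relative location by a fixed step scaled by Rate.
; Pans follow the camera's relative right or up vector.
; Stopping possession halts animation, then after a short delay restores the location and FOV cached at BeginPlay and clears the timer.
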(event `self.ReceiveBeginPlay`
  (set `self.CurrentRelativeLoc` (`self.RelativeLocation`))
  (set `self.CurrentFOV` (`self.FieldOfView`)))

(event `UpdateCamera`
  (bind _relativerotation (`self.RelativeRotation`))
  (bind _simpleanimationtype (`self.SimpleAnimationType`))
  (bind _returnvalue (`KismetMathLibrary.GetRightVector` _relativerotation))
  (bind _returnvalue_2 (`KismetMathLibrary.GetUpVector` _relativerotation))
  (if (`self.Animate`)
    (`|ExecutionSequence`
      (:`then_0`
        (if (`|EnumEquality` _simpleanimationtype "NewEnumerator4")
          (`self.SetFieldOfView` (- (`self.FieldOfView`) (* 0.1 (`self.Rate`))))
          (elif (not (`|EnumEquality` _simpleanimationtype "NewEnumerator5"))
            (`self.K2_SetRelativeLocation` (+ (`self.RelativeLocation`) (* (* (select `/Game/StoryFramework/Core/Blueprints/Enumerators/DialogueCamAnimType_E` (`self.SimpleAnimationType`) :`NewEnumerator0` (* _returnvalue -1.0) :`NewEnumerator1` _returnvalue :`NewEnumerator2` _returnvalue_2 :`NewEnumerator3` (* _returnvalue_2 -1.0)) 0.1) (`self.Rate`))))))))))

(event `OnPossessed`
  (set `self.Animate` true)
  (`KismetSystemLibrary.K2_SetTimer` null "UpdateCamera" (`GameplayStatics.GetWorldDeltaSeconds`) true))

(event `StopPossession`
  (set `self.Animate` false)
  (`KismetSystemLibrary.Delay` 0.1)
  (`self.K2_SetRelativeLocation` (`self.CurrentRelativeLoc`))
  (`self.SetFieldOfView` (`self.CurrentFOV`))
  (`KismetSystemLibrary.K2_ClearTimer` null "UpdateCamera"))