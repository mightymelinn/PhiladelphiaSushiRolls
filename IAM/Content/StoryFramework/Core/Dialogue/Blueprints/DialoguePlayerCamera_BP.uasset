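; Dialogue camera actor for the StoryFramework that stages the player when its owning conversation starts.
; It teleports the player to an optional camera-relative position, then points control rotation at the target NPC's head socket or actor location.
; An optional looping timer drives a timeline that lerps toward random offsets from the original rotation for subtle shake.
; The construction script draws a spline to the NPC matching its assigned ID.
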(event `SlightCameraShake`
  (bind _shakeamount (`self.ShakeAmount`))
  (bind _returnvalue (* _shakeamount -1.0))
  (set `self.RandomAdditiveRotation` (`KismetMathLibrary.MakeRotator` (+ (.roll (`self.OriginalCameraRotation`)) (`KismetMathLibrary.RandomFloatInRange` _returnvalue _shakeamount)) (+ (.pitch (`self.OriginalCameraRotation`)) (`KismetMathLibrary.RandomFloatInRange` _returnvalue _shakeamount)) (+ (.yaw (`self.OriginalCameraRotation`)) (`KismetMathLibrary.RandomFloatInRange` _returnvalue _shakeamount))))
  (bind (_direction _alpha) (`Timeline|CameraShakeAnim` :!via `PlayFromStart`) ; Lerp between randomized rotations.
    (:`Update`
      (`self.K2_SetActorRotation` (`KismetMathLibrary.RLerp` (`self.K2_GetActorRotation`) (`self.RandomAdditiveRotation`) _alpha true)))))

(event `self.ReceiveBeginPlay`
  (if (`self.EnableCameraShake`)
    (set `self.OriginalCameraRotation` (`self.K2_GetActorRotation`))
    (`KismetSystemLibrary.K2_SetTimer` null "SlightCameraShake" 0.1 true)))

(event `OnIDOwnerStartConversation`
  (bind (_returnvalue _istargetvalid) (`self.FindCameraLookAtRotation`))
  (bind _returnvalue_2 (`GameplayStatics.GetPlayerCharacter` 0))
  (bind _setplayerlocation (`self.SetPlayerLocation`))
  ;[0.04314 0.04314 0.05098] Set player location/rotation
  (if (`KismetMathLibrary.NotEqualExactly_VectorVector` _setplayerlocation)
    (`self.K2_SetActorLocation` _returnvalue_2 (`/Game/StoryFramework/Core/Blueprints/BlueprintLibraries/SFGeneralFunctions_BFL.ConvertActorLocalToWorldLcation` _setplayerlocation self) false false)
    (set `self.PreviousUseControllerYaw` (`Pawn.bUseControllerRotationYaw` _returnvalue_2))
    (set `Pawn.bUseControllerRotationYaw` false _returnvalue_2)
    (if _istargetvalid
      (`Controller.SetControlRotation` (`GameplayStatics.GetPlayerController` 0) _returnvalue)
      (set `Pawn.bUseControllerRotationYaw` (`self.PreviousUseControllerYaw`) _returnvalue_2)
      (`Controller.SetIgnoreLookInput` (`GameplayStatics.GetPlayerController` 0) false))))

(fn `FindCameraLookAtRotation`
  (returns (ReturnValue :type "Rotator Structure") (IsTargetValid :type Boolean))
  (bind _targetnpcactor (`/Game/StoryFramework/Core/Blueprints/Components/Core/SFInteractionManager_AC.TargetNPCActor` (`/Game/StoryFramework/Core/Blueprints/BlueprintLibraries/SFGameplayFunctions_BFL.GetSFInteractionManager (Controller)`)))
  (bind _returnvalue (`self.GetComponentByClass` _targetnpcactor "/Script/Engine.SkeletalMeshComponent"))
  (`/Engine/EditorBlueprintResources/StandardMacros.IsValid` _targetnpcactor
    (:`Is Valid`
      (`/Engine/EditorBlueprintResources/StandardMacros.IsValid` _returnvalue
        (:`Is Valid`
          (return (`KismetMathLibrary.FindLookAtRotation` (`PlayerCameraManager.GetCameraLocation` (`GameplayStatics.GetPlayerCameraManager` 0)) (`SceneComponent.GetSocketLocation` _returnvalue "head")) true))
        (:`Is Not Valid`
          (return (`KismetMathLibrary.FindLookAtRotation` (`PlayerCameraManager.GetCameraLocation` (`GameplayStatics.GetPlayerCameraManager` 0)) (`self.K2_GetActorLocation` _targetnpcactor)) true))))
    (:`Is Not Valid`
      (return (struct) false))))

(fn `UserConstructionScript`
  (bind _foundnpc (`/Game/StoryFramework/Core/Blueprints/BlueprintLibraries/SFGameplayFunctions_BFL.GetTargetNPCByID` (`self.AssignToID`)))
  (`SplineComponent.ClearSplinePoints` (`self.IDOwnerPointer`) true)
  (`/Engine/EditorBlueprintResources/StandardMacros.IsValid` _foundnpc
    (:`Is Valid`
      (`SplineComponent.SetSplinePoints` (`self.IDOwnerPointer`) (`|MakeArray` (`self.K2_GetActorLocation`) (`self.K2_GetActorLocation` _foundnpc)) "World" true))
    (:`Is Not Valid`
      (`SceneComponent.SetVisibility` (`self.IDOwnerPointer`) false false))))