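; Example Story Framework NPC that the player can talk to through its dialogue manager component.
; Interface functions supply its talk prompt, dialogue component and NPC info, and interacting starts the conversation.
; Custom action events demonstrate dialogue-driven rewards: a book gift with sound and popup, plus a removable map-puzzle step that tags an NPC SoftLocked and grants an item.
; BeginPlay optionally starts a LookAt timeline for smoothly turning toward the player.
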(event `BobGiveItem`
  ;[0.04314 0.04314 0.05098] Example "Custom Action".
  (`/Game/StoryFramework/Core/Blueprints/BlueprintLibraries/SFGameplayFunctions_BFL.PlaySound2D FromSFV` "OnMemoirNotify")
  (`/Game/StoryFramework/Core/Blueprints/Components/Core/SFInventoryManager_AC.AddItemToInventory` (`/Game/StoryFramework/Core/Blueprints/BlueprintLibraries/SFGameplayFunctions_BFL.GetSFInventoryManager (Controller)`) (make `/Game/StoryFramework/Core/Blueprints/Structures/InteractableData_S` :`ObjectName` "Secret Book" :`ObjectStaticMesh` "/Game/StoryFramework/Core/Example/Level/LevelMeshes/Custom/Book_SM.Book_SM" :`PickupMethodSettings` (make `/Game/StoryFramework/Core/Blueprints/Structures/IMPickupSettings_S` :`ItemInventoryIcon` "/Game/StoryFramework/Core/UserInterface/Textures/BookIcon_T.BookIcon_T" :`CanDrop` false) :`InspectMethodSettings` (make `/Game/StoryFramework/Core/Blueprints/Structures/IMInspectSettings_S` :`InspectMethod` "NewEnumerator1" :`3DInspectActorDistanceFromCamera` 75.0)) 1 null)
  (bind _returnvalue (`|CreateWidget` "/Game/StoryFramework/Core/UserInterface/Widgets/PopupMaster_W.PopupMaster_W_C"))
  (`/Game/StoryFramework/Core/UserInterface/Widgets/PopupMaster_W.ShowCustomPopup` _returnvalue "Bobs Gift" "Bob gave you a book" "/Game/StoryFramework/Core/UserInterface/Textures/InventoryIcon_T.InventoryIcon_T" 5.0 false)
  (`UserWidget.AddToViewport` _returnvalue 0))

(event `self.ReceiveBeginPlay`
  (if (`self.LookAtPlayer`)
    (`/Engine/EditorBlueprintResources/StandardMacros.IsValid` (`GameplayStatics.GetPlayerCharacter` 0)
      (:`Is Valid`
        (`TimelineComponent.Play` (`self.LookAt`))))))

(event `/Game/StoryFramework/Core/Blueprints/BlueprintInterfaces/SFInteraction_BPI.InteractWith`
  (params (DataString :type String))
  (`/Game/StoryFramework/Core/Dialogue/Blueprints/DialogueManager_AC.StartConversation` (`self.NPCDialogueManager`)))

(event `/Game/StoryFramework/Core/Blueprints/BlueprintInterfaces/DialogueInfo_BPI.UpdateOwnerDialogueData`
  (params (NPCInfo :type "/Game/StoryFramework/Core/Blueprints/Structures/NPCBasicInfo_S Structure"))
  (set `self.NPCInfo` NPCInfo))

(event `SecretStepEvent`
  ;[0.04314 0.04314 0.05098] Part of the Example Map Puzzle (Can be removed)
  (bind _outactors (`GameplayStatics.GetAllActorsWithTag` "SecretNPC"))
  (`KismetArrayLibrary.Array_Add` (`Actor.Tags` (`|GetArrayItem` _outactors)) "SoftLocked")
  (`/Game/StoryFramework/Core/Blueprints/Components/Core/SFInventoryManager_AC.AddItemToInventory` (`/Game/StoryFramework/Core/Blueprints/BlueprintLibraries/SFGameplayFunctions_BFL.GetSFInventoryManager (Controller)`) (make `/Game/StoryFramework/Core/Blueprints/Structures/InteractableData_S` :`ObjectName` "Override Sequence" :`PickupMethodSettings` (make `/Game/StoryFramework/Core/Blueprints/Structures/IMPickupSettings_S` null false false false)) 1 null))

(fn `GetInteractionData`
  (returns (InteractionData :type "/Game/StoryFramework/Core/Blueprints/Structures/InteractableData_S Structure"))
  (return (make `/Game/StoryFramework/Core/Blueprints/Structures/InteractableData_S` (`.DisplayName_8_4544C5D1428C67D92B8D84BA105A6AD1` (break `/Game/StoryFramework/Core/Blueprints/Structures/NPCBIName_S` (`.NameInfo_15_5EBED67B48685247F75CBE8C29A24478` (break `/Game/StoryFramework/Core/Blueprints/Structures/NPCBasicInfo_S` (`self.NPCInfo`))))) null null (`self.InteractionPromptOffset`) (`self.DisplayPromptFromRange`) (make `/Game/StoryFramework/Core/Blueprints/Structures/InteractionMethods_S` "NewEnumerator0" "NewEnumerator0" "Talk" null) (struct :`CanDrop` true) (struct) (struct :`InspectMethod` "NewEnumerator0" :`InspectActorOffset` (0.0 0.0 0.0) :`ReadableTextColor` (struct :`SpecifiedColor` (struct :`R` 1.0 :`B` 1.0 :`A` 1.0) :`ColorUseRule` "UseColor_Specified")) (struct :`EffectedAxis` (0.0 1.0 0.0) :`DragSpeedMulti` 1.0 :`DistanceFromOrigin` (struct) :`FocusCameraMode` "NewEnumerator0"))))

(fn `GetOwnerDialogueComponent`
  (returns (DialogueManager :type "/Game/StoryFramework/Core/Dialogue/Blueprints/DialogueManager_AC Object Reference"))
  (return (`self.NPCDialogueManager`)))

(fn `GetOwnerDialogueData`
  (returns (NPCInfo :type "/Game/StoryFramework/Core/Blueprints/Structures/NPCBasicInfo_S Structure"))
  (return (`self.NPCInfo`)))

(fn `UserConstructionScript`)